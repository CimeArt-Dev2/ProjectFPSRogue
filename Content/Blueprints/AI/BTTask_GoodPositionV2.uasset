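; Behavior tree task that positions a BP_Enemy at attack distance from the player.
; Each tick, GoodLocation checks a static-world line trace and distance bands, feeding the InRange key and a navmesh-projected goal: hold, close in when blocked or far, otherwise back off.
; When very close it runs, facing the goal.
; Otherwise it walks facing the player, calls StartAttack even if out of range, and finishes when Attacking is false.
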(event EventReceiveTickAI
  (params (OwnerController :type AI%20Controller%20Object%20Reference) (ControlledPawn :type Pawn%20Object%20Reference) (DeltaSeconds :type Float%20%28single-precision%29))
  (bind _asbp_enemy (Utilities|Casting|CastToBP_Enemy ControlledPawn))
  (bind _playeractor (Variables|Default|GetPlayerActor))
  (bind _returnvalue (AI|BehaviorTree|GetBlackboardValueasActor _playeractor))
  (Variables|Default|SetDelta DeltaSeconds)
  (Variables|Default|SetController OwnerController)
  (Variables|Default|SetEnemy _asbp_enemy)
  (Variables|Default|SetEnemyLocation (Transformation|GetActorLocation _asbp_enemy))
  (Utilities|IsValid _returnvalue
    (:Is%20Valid
      (Variables|Default|SetPlayerLocation (Transformation|GetActorLocation _returnvalue))
      (Pawn|SetControlRotation (Variables|Default|GetController) (Math|Rotator|FindLookatRotation (Variables|Default|GetEnemyLocation) (Variables|Default|GetPlayerLocation)))
      (Development|PrintString (Utilities|String|ToString(Rotator) (Math|Rotator|FindLookatRotation (Variables|Default|GetEnemyLocation) (Variables|Default|GetPlayerLocation)))))
    (:Is%20Not%20Valid
      _))
  (Class|BTFunctionLibrary|SetBlackboardValueasBool (Variables|Default|GetInRange?) (or (.GoodLocation (CallFunction|GoodLocation? (Variables|Default|GetEnemyLocation) (Variables|Default|GetPlayerLocation))) (.TooClose (CallFunction|GoodLocation? (Variables|Default|GetEnemyLocation) (Variables|Default|GetPlayerLocation)))))
  (if (.TooClose (CallFunction|GoodLocation? (Variables|Default|GetEnemyLocation) (Variables|Default|GetPlayerLocation)))
    (Variables|/Script/Engine.CharacterMovementComponent|SetMaxWalkSpeed (Variables|/Script/Engine.Character|GetCharacterMovement (Variables|Default|GetEnemy)) 6e+02)
    (AI|Navigation|SimpleMovetoLocation (Variables|Default|GetController) (.ProjectedLocation (AI|Navigation|ProjectPointtoNavigation (select (.GoodLocation (CallFunction|GoodLocation? (Variables|Default|GetEnemyLocation) (Variables|Default|GetPlayerLocation))) (Variables|Default|GetEnemyLocation) (+ (Variables|Default|GetEnemyLocation) (* (* (Math|Vector|GetUnitDirection(Vector) (Variables|Default|GetPlayerLocation) (Variables|Default|GetEnemyLocation)) (select (or (.Wall (CallFunction|GoodLocation? (Variables|Default|GetEnemyLocation) (Variables|Default|GetPlayerLocation))) (.Too%20far (CallFunction|GoodLocation? (Variables|Default|GetEnemyLocation) (Variables|Default|GetPlayerLocation)))) -1 1)) (/ (Variables|Default|GetMaxDistance) 2.0)))) 0 0 "2000.000000,2000.000000,2000.000000")))
    (Pawn|SetControlRotation (Variables|Default|GetController) (Math|Rotator|FindLookatRotation (Variables|Default|GetEnemyLocation) (.ProjectedLocation (AI|Navigation|ProjectPointtoNavigation (select (.GoodLocation (CallFunction|GoodLocation? (Variables|Default|GetEnemyLocation) (Variables|Default|GetPlayerLocation))) (Variables|Default|GetEnemyLocation) (+ (Variables|Default|GetEnemyLocation) (* (* (Math|Vector|GetUnitDirection(Vector) (Variables|Default|GetPlayerLocation) (Variables|Default|GetEnemyLocation)) (select (or (.Wall (CallFunction|GoodLocation? (Variables|Default|GetEnemyLocation) (Variables|Default|GetPlayerLocation))) (.Too%20far (CallFunction|GoodLocation? (Variables|Default|GetEnemyLocation) (Variables|Default|GetPlayerLocation)))) -1 1)) (/ (Variables|Default|GetMaxDistance) 2.0)))) 0 0 "2000.000000,2000.000000,2000.000000"))))
    (else
      (Variables|/Script/Engine.CharacterMovementComponent|SetMaxWalkSpeed (Variables|/Script/Engine.Character|GetCharacterMovement (Variables|Default|GetEnemy)) 3e+02)
      (AI|Navigation|SimpleMovetoLocation (Variables|Default|GetController) (.ProjectedLocation (AI|Navigation|ProjectPointtoNavigation (select (.GoodLocation (CallFunction|GoodLocation? (Variables|Default|GetEnemyLocation) (Variables|Default|GetPlayerLocation))) (Variables|Default|GetEnemyLocation) (+ (Variables|Default|GetEnemyLocation) (* (* (Math|Vector|GetUnitDirection(Vector) (Variables|Default|GetPlayerLocation) (Variables|Default|GetEnemyLocation)) (select (or (.Wall (CallFunction|GoodLocation? (Variables|Default|GetEnemyLocation) (Variables|Default|GetPlayerLocation))) (.Too%20far (CallFunction|GoodLocation? (Variables|Default|GetEnemyLocation) (Variables|Default|GetPlayerLocation)))) -1 1)) (/ (Variables|Default|GetMaxDistance) 2.0)))) 0 0 "2000.000000,2000.000000,2000.000000")))
      (Pawn|SetControlRotation (Variables|Default|GetController) (Math|Rotator|FindLookatRotation (Variables|Default|GetEnemyLocation) (Variables|Default|GetPlayerLocation)))
      (Default|StartAttack (Variables|Default|GetEnemy))
      (if (not (Variables|/Game/Blueprints/AI/BP_Enemy.BP_Enemy_C|GetAttacking? (Variables|Default|GetEnemy)))
        (AI|BehaviorTree|FinishExecute true)))))

(event EventReceiveExecuteAI
  (params (OwnerController :type AI%20Controller%20Object%20Reference) (ControlledPawn :type Pawn%20Object%20Reference))
  ;[1 1 1] Need Distance Attack
)

(fn GoodLocation?
  (params (EnemyLocation :type Vector) (PlayerLocation :type Vector))
  (bind _returnvalue (Math|Vector|Distance(Vector) EnemyLocation PlayerLocation))
  (bind _maxdistance (Variables|Default|GetMaxDistance))
  (bind _returnvalue_2 (Collision|LineTraceForObjects EnemyLocation PlayerLocation (Utilities|Array|MakeArray "ObjectTypeQuery1") false 0 "None"))
  (return (and (not _returnvalue_2) (Math|Float|InRange(Float) _returnvalue (Variables|Default|GetMinDist) _maxdistance)) _returnvalue_2 (> _returnvalue _maxdistance) (< _returnvalue (Variables|Default|GetRealyCloseDistance))))