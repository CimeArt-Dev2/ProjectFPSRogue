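; Behavior tree service that picks an AI target location near the player, kept at a minimum distance from them.
; On activation it samples a random reachable navigation point within a radius around the blackboard's player actor.
; The point is written to the target location key only if far enough from the player, with no retry otherwise.
; It also prints the distance check on screen for debugging.
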(event EventReceiveActivationAI
  (params (OwnerController :type AI%20Controller%20Object%20Reference) (ControlledPawn :type Pawn%20Object%20Reference))
  (bind _minimaldistance (Variables|Default|GetMinimalDistance))
  (bind _playeractor (Variables|Default|GetPlayerActor))
  (bind _returnvalue (AI|BehaviorTree|GetBlackboardValueasActor _playeractor))
  (bind _returnvalue_2 (Transformation|GetActorLocation _returnvalue))
  (bind _output_get (Variables|Default|SetCalculatedLocation (.RandomLocation (AI|Navigation|GetRandomReachablePointinRadius _returnvalue_2 (Variables|Default|GetRadius) 0 0))))
  (Development|PrintString (Utilities|String|Append (Utilities|String|ToString(Float) (Math|Vector|Distance(Vector) _output_get _returnvalue_2)) ">=" (Utilities|String|ToString(Float) _minimaldistance) " = " (Utilities|String|ToString(Boolean) (>= (Math|Vector|Distance(Vector) _output_get _returnvalue_2) _minimaldistance))) true true "(R=0.000000,G=0.660000,B=1.000000,A=1.000000)" 1e+01)
  (if (>= (Math|Vector|Distance(Vector) _output_get _returnvalue_2) _minimaldistance)
    (AI|BehaviorTree|SetBlackboardValueasVector (Variables|Default|GetTargetLocationKey) (Variables|Default|GetCalculatedLocation))))