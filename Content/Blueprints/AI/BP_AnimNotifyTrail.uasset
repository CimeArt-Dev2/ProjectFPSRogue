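; Anim notify state that detects enemy melee hits during an attack animation.
; Each tick, it sphere-traces for pawns between the LeftHand and LeftHandSocket sockets, with debug drawing left visible for a duration.
; A hit TestAnimWeapon actor takes the owning BP_Enemy's Damage, and the enemy's PlayerHit flag is set to block repeat hits; this file never resets that flag.
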(fn ReceivedNotifyTick
  (params (MeshComp :type Skeletal%20Mesh%20Component%20Object%20Reference) (Animation :type Anim%20Sequence%20Base%20Object%20Reference) (FrameDeltaTime :type Float%20%28single-precision%29))
  (bind _returnvalue (Components|GetOwner MeshComp))
  (bind _asbp_enemy (Utilities|Casting|CastToBP_Enemy _returnvalue))
  (bind _outhit (Collision|SphereTraceForObjects MeshComp (Transformation|GetSocketLocation MeshComp "LeftHand") (Transformation|GetSocketLocation MeshComp "LeftHandSocket") 3e+01 (Utilities|Array|MakeArray "ObjectTypeQuery3") false 0 "ForDuration"))
  (bind _astest_anim_weapon (Utilities|Casting|CastToTestAnimWeapon (.hitactor _outhit)))
  (if (not (Variables|/Game/Blueprints/AI/BP_Enemy.BP_Enemy_C|GetPlayerHit? _asbp_enemy))
    (Default|TakeDamage _astest_anim_weapon (Variables|/Game/Blueprints/AI/BP_Enemy.BP_Enemy_C|GetDamage _asbp_enemy))
    (Variables|/Game/Blueprints/AI/BP_Enemy.BP_Enemy_C|SetPlayerHit? _asbp_enemy true)
    (return false)))