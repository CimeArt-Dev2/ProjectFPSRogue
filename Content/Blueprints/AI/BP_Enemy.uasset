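; Enemy character Blueprint with hit points, an attack trigger and a ragdoll death.
; Construction script tints the mesh's BodyColor material parameter red for Blind enemies and grey-beige otherwise.
; StartAttack forwards AttackMessage to the anim instance, and TakeDamage only subtracts from CurrentHP.
; A separate Death function checks for zero HP, then enables mesh physics with a bone impulse, disables capsule collision, detaches the controller and sets IsDead.
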(event Custom|StartAttack
  (Class|INTAnimBPEnemy|Attack(Message) (Components|SkeletalMesh|GetAnimInstance (Variables|Character|GetMesh))))

(event EventBeginPlay)

(event Collision|EventActorBeginOverlap
  (params (OtherActor :type Actor%20Object%20Reference)))

(event EventTick
  (params (DeltaSeconds :type Float%20%28single-precision%29)))

(fn ConstructionScript
  (Rendering|Material|SetVectorParameterValueonMaterials (Variables|Character|GetMesh) "BodyColor" (Math|Conversions|ToVector(LinearColor) (select (Variables|Default|GetBlind?) "(R=0.645833,G=0.025266,B=0.003364,A=0.000000)" "(R=0.450980,G=0.403922,B=0.360784,A=0.000000)"))))

(fn TakeDamage
  (params (Damage :type Float%20%28single-precision%29))
  (Variables|Default|SetCurrentHP (- (Variables|Default|GetCurrentHP) Damage)))

(fn Death
  (params (Impulse :type Vector) (BoneName :type Name))
  (if (<= (Variables|Default|GetCurrentHP) 0.0)
    (Physics|SetSimulatePhysics (Variables|Character|GetMesh) true)
    (Collision|SetCollisionEnabled (Variables|Collision|GetCapsuleComponent) "NoCollision")
    (Physics|AddImpulse (Variables|Character|GetMesh) Impulse BoneName true)
    (Class|Pawn|DetachfromControllerPendingDestroy)
    (Variables|Default|SetIsDead? true)))