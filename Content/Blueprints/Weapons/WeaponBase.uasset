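; Base weapon Blueprint handling hitscan firing, reloading and per-weapon XP leveling for the TestAnimWeapon first-person character.
; Fire plays animations and line-traces from the camera, damaging living BP_Enemy targets, passing Death an impulse, then delays refiring; knives work without ammo.
; Reload refills from reserve on a montage notify.
; Hits grant XP toward levels with scaling thresholds, and every gain while at certain milestone levels compounds damage by 10%.
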(event Custom|Fire
  ;[1 1 1] Fire
  (if (and (Variables|Default|GetCanFire) (not (Variables|Default|GetIsReloading)))
    (if (> (Variables|Default|GetAmmo) 0)
      (Math|Integer|DecrementInt (Variables|Default|GetAmmo)
        (:%20%20
          (Variables|Default|SetCanFire false :!label _label)
          (Components|Animation|PlayAnimation (Variables|Default|GetSkeletalMesh) (Variables|Default|GetAnimPlayWeapon) false)
          (bind _astest_anim_weapon (Utilities|Casting|CastToTestAnimWeapon (Game|GetPlayerCharacter 0)))
          (Animation|Montage|MontagePlay (Components|SkeletalMesh|GetAnimInstance (Variables|/Game/Blueprints/Player/TestAnimWeapon.TestAnimWeapon_C|GetMesh2P _astest_anim_weapon)) (Variables|Default|GetAnimPlayArms) 1.0 "MontageLength" 0.0 true)
          (CallFunction|LineTraceDamage)))
      (elif (Utilities|Name|Equal(Name) (Variables|Default|Getname) "knife")
        (goto _label)))))

(event Custom|LineTraceDamage
  ;[1 1 1] LineTrace Damage
  (bind _astest_anim_weapon (Utilities|Casting|CastToTestAnimWeapon (Game|GetPlayerCharacter 0)))
  (bind _outhit (Collision|LineTraceByChannel (Transformation|GetWorldLocation (Variables|/Game/Blueprints/Player/TestAnimWeapon.TestAnimWeapon_C|GetFirstPersonCamera _astest_anim_weapon)) (+ (Transformation|GetWorldLocation (Variables|/Game/Blueprints/Player/TestAnimWeapon.TestAnimWeapon_C|GetFirstPersonCamera _astest_anim_weapon)) (* (Math|Vector|GetForwardVector (Variables|/Game/Blueprints/Player/TestAnimWeapon.TestAnimWeapon_C|GetFirstPersonCamera _astest_anim_weapon)) (Variables|Default|GetFireDistance))) "TraceTypeQuery1" false 0 "ForDuration"))
  (bind _asbp_enemy (Utilities|Casting|CastToBP_Enemy (.hitactor _outhit))
    (:then
      (if (Variables|/Game/Blueprints/AI/BP_Enemy.BP_Enemy_C|GetIsDead? _asbp_enemy)
        _
        (else
          (Default|TakeDamage _asbp_enemy (Variables|Default|GetDamage))
          (Default|Death _asbp_enemy (* (Math|Vector|GetForwardVector (Variables|/Game/Blueprints/Player/TestAnimWeapon.TestAnimWeapon_C|GetFirstPersonCamera _astest_anim_weapon)) (Variables|/Game/Blueprints/Player/TestAnimWeapon.TestAnimWeapon_C|GetImpulseShot _astest_anim_weapon)) (.hitbonename _outhit))
          (CallFunction|AddXP 1e+01))))
    (:CastFailed
      _))
  (Utilities|FlowControl|Delay (Variables|Default|GetDelayFire))
  (Variables|Default|SetCanFire true))

(event Custom|Reload
  ;[1 1 1] Reload
  (bind _astest_anim_weapon (Utilities|Casting|CastToTestAnimWeapon (Game|GetPlayerCharacter 0)))
  (if (Math|Boolean|ANDBoolean (< (Variables|Default|GetAmmo) (Variables|Default|GetMaxAmmo)) (> (Variables|Default|GetChargeur) 0) (not (Variables|Default|GetIsReloading)))
    (Utilities|FlowControl|DoOnce false :!label _label
      (:Completed
        (Variables|Default|SetIsReloading true)
        (bind _notifyname (Animation|Montage|PlayMontage (Variables|/Game/Blueprints/Player/TestAnimWeapon.TestAnimWeapon_C|GetMesh2P _astest_anim_weapon) (Variables|Default|GetAnimPlayReloading))
          (:OnNotifyBegin
            (if (Utilities|Name|Equal(Name) _notifyname "Reloading")
              (Variables|Default|SetBufferAmmo (- (Variables|Default|GetMaxAmmo) (Variables|Default|GetAmmo)))
              (if (< (Variables|Default|GetChargeur) (Variables|Default|GetBufferAmmo))
                (Variables|Default|SetAmmo (+ (Variables|Default|GetAmmo) (Variables|Default|GetChargeur)))
                (Variables|Default|SetChargeur 0)
                (else
                  (Variables|Default|SetChargeur (- (Variables|Default|GetChargeur) (Variables|Default|GetBufferAmmo)))
                  (Variables|Default|SetAmmo (Variables|Default|GetMaxAmmo))))
              (Variables|Default|SetIsReloading false)
              (goto _label Reset))))))
    (else
      (goto _label Reset))))

(fn ConstructionScript)

(fn LevelUP
  (if (>= (Variables|Default|GetCurrentXP) (Variables|Default|GetMaxXP))
    (if (< (Variables|Default|GetCurrentLevel) (Variables|Default|GetMaxLevel))
      (Math|Integer|IncrementInt (Variables|Default|GetCurrentLevel)
        (:%20%20
          (Variables|Default|SetCurrentXP 0.0)
          (Variables|Default|SetMaxXP (* (Variables|Default|GetMaxXP) (Variables|Default|GetUpMaxXP))))))))

(fn AddXP
  (params (A :type Float%20%28single-precision%29))
  (Variables|Default|SetCurrentXP (+ A (Variables|Default|GetCurrentXP)))
  (CallFunction|LevelUP)
  (if (Math|Boolean|ORBoolean (== (Variables|Default|GetCurrentLevel) 5) (== (Variables|Default|GetCurrentLevel) 10) (== (Variables|Default|GetCurrentLevel) 15) (== (Variables|Default|GetCurrentLevel) 20))
    (CallFunction|DamageUP)))

(fn DamageUP
  (Variables|Default|SetUPDamage (/ (* (Variables|Default|GetDamage) 1e+01) 1e+02))
  (Variables|Default|SetDamage (+ (Variables|Default|GetDamage) (Variables|Default|GetUPDamage))))