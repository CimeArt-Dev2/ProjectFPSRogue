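; BP_PNJ is a configurable HUB NPC that can open a dialogue with the player.
; The construction script uses the Who enum as a row name in DT_PNJ to set the skeletal mesh, anim class, vertical mesh offset and dialogues, so one Blueprint serves every character.
; LaunchDialogues creates a DemoDialogueWidget, passing those dialogues and the NPC itself.
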(event Custom|LaunchDialogues
  (UserInterface|CreateWidget "/DialoguePlugin/UI/DemoDialogueWidget.DemoDialogueWidget_C" 0 (Variables|Default|GetDialogues) self))

(fn ConstructionScript
  (bind _mesh (Variables|Character|GetMesh))
  (bind _returnvalue (Utilities|GetDataTableRow "/Game/Blueprints/HUB/Dialogues/DT_PNJ.DT_PNJ" (Utilities|String|StringToName (Utilities|String|EnumtoString (Variables|Default|GetWho?))))
    (:then
      (Class|SkinnedMeshComponent|SetSkeletalMesh (Variables|Character|GetMesh) (.skeletal _returnvalue) true)
      (Variables|Default|SetDialogues (.dialogues _returnvalue))
      (Class|SkeletalMeshComponent|SetAnimClass _mesh (.anim _returnvalue))
      (Transformation|SetRelativeLocation _mesh (Math|Vector|MakeVector 0.0 0.0 (* (.height _returnvalue) -1.0)) false false))))