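; BP_Object_Dialogues is a hub object that opens a dialogue widget when its LaunchDialogues event fires.
; Its construction script uses the What enum as a row name in DT_Object_Dialogues to set the static mesh, its height and the dialogue data.
; LaunchDialogues creates a DemoDialogueWidget with that data and passes the object itself as the NPC actor.
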(event Custom|LaunchDialogues
  (UserInterface|CreateWidget "/DialoguePlugin/UI/DemoDialogueWidget.DemoDialogueWidget_C" 0 (Variables|Default|GetDialogues) self))

(fn ConstructionScript
  (bind _staticmesh (Variables|Default|GetStaticMesh))
  (bind _returnvalue (Utilities|GetDataTableRow "/Game/Blueprints/HUB/Dialogues/DT_Object_Dialogues.DT_Object_Dialogues" (Utilities|String|StringToName (Utilities|String|EnumtoString (Variables|Default|GetWhat?))))
    (:then
      (Components|StaticMesh|SetStaticMesh _staticmesh (.mesh _returnvalue))
      (Variables|Default|SetDialogues (.dialogues _returnvalue))
      (Transformation|SetRelativeLocation _staticmesh (Math|Vector|MakeVector 0.0 0.0 (.height _returnvalue)) false false))))